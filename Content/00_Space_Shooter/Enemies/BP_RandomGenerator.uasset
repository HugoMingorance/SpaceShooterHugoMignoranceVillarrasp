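; BP_RandomGenerator is the space shooter's enemy spawner, creating a random enemy on a looping timer.
; Each spawn draws a random index below the game mode's Level and clamps it to pick one of four enemy classes, so higher levels widen the possible variety.
; The enemy appears at a randomly chosen scene component on the spawner tagged SpawnPoint.
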(event Custom|Spawn
  (CallFunction|SpawnEnemy))

(event EventBeginPlay
  (Utilities|Time|SetTimerbyEvent (delegate Custom|Spawn) (Variables|Default|Getspaw%20time) true)
  (bind _asss_game_mode (Utilities|Casting|CastToSS_GameMode (Game|GetGameMode)))
  (Variables|Default|SetSS_GM _asss_game_mode))

(event Collision|EventActorBeginOverlap
  (params (OtherActor :type Actor%20Object%20Reference)))

(event EventTick
  (params (DeltaSeconds :type Float%20%28single-precision%29)))

(fn ConstructionScript)

(fn SpawnEnemy
  (bind _returnvalue (Actor|GetComponentsbyTag "/Script/Engine.SceneComponent" "SpawnPoint"))
  (bind _newparam (CallFunction|GetClasstoSpawn (Math|Random|RandomInteger (Variables|/Game/00_Space_Shooter/SS_GameMode.SS_GameMode_C|Getlevel (Variables|Default|GetSS_GM)))))
  (Game|SpawnActorfromClass _newparam (Transformation|GetWorldTransform (Utilities|Array|Get(acopy) _returnvalue (Math|Random|RandomInteger (Utilities|Array|Length _returnvalue)))) "Undefined" "MultiplyWithRoot" 0 0))

(fn GetClasstoSpawn
  (params (Type :type Integer))
  (return (Utilities|Select :Index (Math|Integer|Clamp(Integer) Type 0 3) :Option%200 "/Game/00_Space_Shooter/Enemies/BP_EnemyBase.BP_EnemyBase_C" :Option%201 "/Game/00_Space_Shooter/Enemies/BP_EnemyH.BP_EnemyH_C" :Option%202 "/Game/00_Space_Shooter/Enemies/Kamikaze_enemy.Kamikaze_enemy_C" :Option%203 "/Game/00_Space_Shooter/Enemies/LaserEnemy.LaserEnemy_C")))